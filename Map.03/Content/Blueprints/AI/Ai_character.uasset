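; AI character Blueprint that wanders the navmesh and moves toward pawns it sees.
; On BeginPlay a Roam loop moves it to random reachable points within a radius of its location, repeating after a short delay on each successful arrival.
; PawnSensing sightings start a move to the seen pawn and refresh a retriggerable delay, which resumes roaming shortly after sightings stop.
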(event `self.ReceiveTick`
  (params (DeltaSeconds :type "Float (single-precision)")))

(event `self.ReceiveBeginPlay`
  (`self.Roam`))

(event `self.PawnSensing.OnSeePawn`
  (params (Pawn :type "Pawn Object Reference"))
  (`|ExecutionSequence`
    (:`then_0`
      (`|AIMoveTo` self (0.0 0.0 0.0) Pawn))
    (:`then_1`
      (`KismetSystemLibrary.RetriggerableDelay` 0.5)
      (`self.Roam`))))

(event `Roam`
  (`|AIMoveTo` self (`NavigationSystemV1.K2_GetRandomReachablePointInRadius` (`self.K2_GetActorLocation`) 1500.0 null null) null
    (:`OnSuccess`
      (`KismetSystemLibrary.Delay` 0.2)
      (`self.Roam` self))))

(fn `UserConstructionScript`)